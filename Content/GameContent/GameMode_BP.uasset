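; Game mode Blueprint that tracks how many cars are inside and checks the win condition.
; AddCar and RemoveCar raise or lower CurrentCarsInside, then share one check against TotalNumCarsToWin.
; The check only prints an on-screen Spanish message, green for a win or red for not yet won, with no further game-over logic.
; BeginPlay, Tick and the construction script are empty.
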(event Custom|AddCar
  (Math|Integer|IncrementInt (Variables|Default|GetCurrentCarsInside)
    (:%20%20
      (if (>= (Variables|Default|GetCurrentCarsInside) (Variables|Default|GetTotalNumCarsToWin))
        (Development|PrintString "Has ganado" true true "(R=0.163937,G=1.000000,B=0.173954,A=1.000000)" 1e+01)
        (else
          (Development|PrintString "Todavia no has ganado" true true "(R=1.000000,G=0.047707,B=0.000000,A=1.000000)" 1.0))))))

(event Custom|RemoveCar
  (Math|Integer|DecrementInt (Variables|Default|GetCurrentCarsInside)
    (:%20%20
      (if (>= (Variables|Default|GetCurrentCarsInside) (Variables|Default|GetTotalNumCarsToWin))
        (Development|PrintString "Has ganado" true true "(R=0.163937,G=1.000000,B=0.173954,A=1.000000)" 1e+01)
        (else
          (Development|PrintString "Todavia no has ganado" true true "(R=1.000000,G=0.047707,B=0.000000,A=1.000000)" 1.0))))))

(event EventBeginPlay)

(event EventTick
  (params (DeltaSeconds :type Float%20%28single-precision%29)))

(fn ConstructionScript)