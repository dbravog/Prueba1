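; ShipCar_BP is a player-controlled flying vehicle pawn, apparently a ship-car, with a third-person camera.
; Input axes feed AddMovementInput: forward and vertical movement follow fixed world X and Z from zero rotations, while strafing follows the actor's right vector.
; Mouse axes drive controller yaw and pitch, and a wheel axis changes the SpringArm length for unclamped zoom.
; Tick and the construction script are empty.
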(event EventTick
  (params (DeltaSeconds :type Float%20%28single-precision%29))
  ;[1 1 1] Movimiento
)

(event Input|AxisEvents|InputAxisMoveUpDown
  (params (AxisValue :type Float%20%28single-precision%29))
  ;[1 1 1] Movimiento
  (Pawn|Input|AddMovementInput (Math|Vector|GetUpVector "0, 0, 0") AxisValue false))

(event Input|AxisEvents|InputAxisRuedaZoom
  (params (AxisValue :type Float%20%28single-precision%29))
  (bind _springarm (Variables|Default|GetSpringArm))
  ;[1 1 1] Camara 3ª Persona
  (Variables|/Script/Engine.SpringArmComponent|SetTargetArmLength _springarm (+ (* AxisValue 1e+01) (Variables|/Script/Engine.SpringArmComponent|GetTargetArmLength _springarm))))

(event Input|AxisEvents|InputAxisMouseHorizontal
  (params (AxisValue :type Float%20%28single-precision%29))
  ;[1 1 1] Camara 3ª Persona
  (Pawn|Input|AddControllerYawInput AxisValue))

(event Input|AxisEvents|InputAxisMouseVertical
  (params (AxisValue :type Float%20%28single-precision%29))
  ;[1 1 1] Camara 3ª Persona
  (Pawn|Input|AddControllerPitchInput AxisValue))

(event Input|AxisEvents|InputAxisMoveVertical
  (params (AxisValue :type Float%20%28single-precision%29))
  ;[1 1 1] Movimiento
  (Pawn|Input|AddMovementInput (Math|Vector|GetForwardVector "0, 0, 0") AxisValue false))

(event Input|AxisEvents|InputAxisMoveHorizontal
  (params (AxisValue :type Float%20%28single-precision%29))
  ;[1 1 1] Movimiento
  (Pawn|Input|AddMovementInput (Transformation|GetActorRightVector) AxisValue false))

(fn ConstructionScript)